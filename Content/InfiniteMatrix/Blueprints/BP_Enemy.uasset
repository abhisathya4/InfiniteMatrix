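; BP_Enemy is an enemy actor with a pill mesh that tumbles on all three axes every tick and hits the player on contact.
; When a BP_Player stops overlapping the pill, it calls that player's ProcessHit.
; It then destroys the enemy referenced by the player's SpawnedEnemy, if valid, rather than itself directly, and sets the player's SpawnEnemyLocation to a fixed point.
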(event `self.ReceiveTick`
  (params (DeltaSeconds :type "Float (single-precision)"))
  (bind _returnvalue (* DeltaSeconds 30.0))
  (`SceneComponent.K2_AddWorldRotation` (`self.Pill Mesh`) (`KismetMathLibrary.MakeRotator` _returnvalue _returnvalue _returnvalue) false false))

(event `self.Pill Mesh.OnComponentEndOverlap`
  (params (OverlappedComponent :type "PrimitiveComponent Object Reference") (OtherActor :type "Actor Object Reference") (OtherComp :type "PrimitiveComponent Object Reference") (OtherBodyIndex :type Integer))
  (bind _asbp_player (cast `/Game/InfiniteMatrix/Blueprints/BP_Player` OtherActor))
  (`/Game/InfiniteMatrix/Blueprints/BP_Player.ProcessHit` _asbp_player)
  (bind _spawnedenemy (`/Game/InfiniteMatrix/Blueprints/BP_Player.SpawnedEnemy` _asbp_player))
  (if (`KismetSystemLibrary.IsValid` _spawnedenemy)
    (`self.K2_DestroyActor` _spawnedenemy)
    (set `/Game/InfiniteMatrix/Blueprints/BP_Player.SpawnEnemyLocation` (-123.0 0.0 0.0) _asbp_player)))

(fn `UserConstructionScript`)