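; BP_Projectile is a shot that flies along world X at ForwardSpeed and kills BP_Enemy actors.
; Tick moves it and destroys it only if a single frame's DeltaSeconds exceeds two seconds, so this is not an accumulated lifetime.
; Mesh overlap with BP_Pill destroys just the projectile.
; An enemy hit, given a valid Player, raises the score, destroys both actors and sets the Player's SpawnEnemyLocation to a fixed point.
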(event `self.ReceiveTick`
  (params (DeltaSeconds :type "Float (single-precision)"))
  (`self.K2_AddActorWorldOffset` (`KismetMathLibrary.MakeVector` (* DeltaSeconds (`self.ForwardSpeed`))))
  (if (> DeltaSeconds 2.0)
    (`self.K2_DestroyActor`)))

(event `self.ProjectileStaticMesh.OnComponentBeginOverlap`
  (params (OverlappedComponent :type "PrimitiveComponent Object Reference") (OtherActor :type "Actor Object Reference") (OtherComp :type "PrimitiveComponent Object Reference") (OtherBodyIndex :type Integer) (bFromSweep :type Boolean) (SweepResult :type "HitResult Structure (by ref)"))
  (bind _player (`self.Player`))
  (cast `/Game/InfiniteMatrix/Blueprints/BP_Pill` OtherActor
    (:`then`
      (`self.K2_DestroyActor`))
    (:`CastFailed`
      (bind _asbp_enemy (cast `/Game/InfiniteMatrix/Blueprints/BP_Enemy` OtherActor))
      (if (`KismetSystemLibrary.IsValid` _player)
        (`/Game/InfiniteMatrix/Blueprints/BP_Player.IncreaseScoreAfterKill` _player)
        (`self.K2_DestroyActor` _asbp_enemy)
        (set `/Game/InfiniteMatrix/Blueprints/BP_Player.SpawnEnemyLocation` (-123.0 0.0 0.0) _player)
        (`self.K2_DestroyActor`)))))

(fn `UserConstructionScript`)